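; Paddles is a two-handed paddle prop that reports a push velocity and origin from whichever blade is in water.
; Left and right spheres gain a "Water" tag while overlapping water body collision, and GetPushVelocity reads it, favoring the left.
; Tick derives velocity from per-frame position deltas, but both passes write the left variables, so right-side values never update here.
; IsHeld requires both grab components to be held.
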(event `self.SphereL.OnComponentBeginOverlap`
  (params (OverlappedComponent :type "PrimitiveComponent Object Reference") (OtherActor :type "Actor Object Reference") (OtherComp :type "PrimitiveComponent Object Reference") (OtherBodyIndex :type Integer) (bFromSweep :type Boolean) (SweepResult :type "HitResult Structure (by ref)"))
  (if (== (`PrimitiveComponent.GetCollisionProfileName` OtherComp) "WaterBodyCollision")
    (`KismetArrayLibrary.Array_Add` (`ActorComponent.ComponentTags` (`self.SphereL`)) "Water")))

(event `self.SphereL.OnComponentEndOverlap`
  (params (OverlappedComponent :type "PrimitiveComponent Object Reference") (OtherActor :type "Actor Object Reference") (OtherComp :type "PrimitiveComponent Object Reference") (OtherBodyIndex :type Integer))
  (if (== (`PrimitiveComponent.GetCollisionProfileName` OtherComp) "WaterBodyCollision")
    (`KismetArrayLibrary.Array_RemoveItem` (`ActorComponent.ComponentTags` (`self.SphereL`)) "Water")))

(event `self.SphereR.OnComponentBeginOverlap`
  (params (OverlappedComponent :type "PrimitiveComponent Object Reference") (OtherActor :type "Actor Object Reference") (OtherComp :type "PrimitiveComponent Object Reference") (OtherBodyIndex :type Integer) (bFromSweep :type Boolean) (SweepResult :type "HitResult Structure (by ref)"))
  (if (== (`PrimitiveComponent.GetCollisionProfileName` OtherComp) "WaterBodyCollision")
    (`KismetArrayLibrary.Array_Add` (`ActorComponent.ComponentTags` (`self.SphereR`)) "Water")))

(event `self.SphereR.OnComponentEndOverlap`
  (params (OverlappedComponent :type "PrimitiveComponent Object Reference") (OtherActor :type "Actor Object Reference") (OtherComp :type "PrimitiveComponent Object Reference") (OtherBodyIndex :type Integer))
  (if (== (`PrimitiveComponent.GetCollisionProfileName` OtherComp) "WaterBodyCollision")
    (`KismetArrayLibrary.Array_RemoveItem` (`ActorComponent.ComponentTags` (`self.SphereR`)) "Water")))

(event `self.ReceiveTick`
  (params (DeltaSeconds :type "Float (single-precision)"))
  (bind _returnvalue (`SceneComponent.K2_GetComponentLocation` (`self.SphereR`)))
  (bind _returnvalue_2 (`SceneComponent.K2_GetComponentLocation` (`self.SphereL`)))
  (`|ExecutionSequence`
    (:`then_0`
      (set `self.SphereLVelocity` (- _returnvalue_2 (`self.LastSphereLLocation`)))
      (set `self.LastSphereLLocation` _returnvalue_2))
    (:`then_1`
      (set `self.SphereLVelocity` (- _returnvalue (`self.LastSphereLLocation`)))
      (set `self.LastSphereLLocation` _returnvalue))))

(fn `GetPushVelocity`
  (returns (Velocity :type "Vector Structure") (Origin :type "Vector Structure"))
  (if (`ActorComponent.ComponentHasTag` (`self.SphereL`) "Water")
    (return (`self.SphereLVelocity`) (`self.LastSphereLLocation`))
    (elif (`ActorComponent.ComponentHasTag` (`self.SphereR`) "Water")
      (return (`self.SphereRVelocity`) (`self.LastSphereRLocation`))
      (else
        (return (0.0 0.0 0.0) (0.0 0.0 0.0))))))

(fn `IsHeld?`
  (returns (`OutIsHeld?` :type Boolean))
  (return (and (`/Game/VRTemplate/Blueprints/GrabComponent.bIsHeld` (`self.GrabComponent`)) (`/Game/VRTemplate/Blueprints/GrabComponent.bIsHeld` (`self.GrabComponent1`)))))

(fn `UserConstructionScript`)