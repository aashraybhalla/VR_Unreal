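; Laser sword actor that detects hits along its blade with sphere traces and calls ApplyDamage on actors it hits.
; Each Tick runs a series of Visibility traces between points interpolated along the current and cached Trace_Start/Trace_End socket positions.
; Trace radius derives from blade length at BeginPlay.
; The cache refreshes inside the loop, so only the first trace sweeps from the previous frame's position.
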(event `self.ReceiveBeginPlay`
  (`self.CacheTraceLoacations`)
  (set `self.TraceStep` (/ (`KismetMathLibrary.Vector_Distance` (`self.LastTraceStartLocation`) (`self.LastTraceEndLocation`)) 20.0)))

(event `self.ReceiveTick`
  (params (DeltaSeconds :type "Float (single-precision)"))
  (bind _staticmesh (`self.StaticMesh`))
  (for _index (range 11)
    (bind _returnvalue (/ (`KismetMathLibrary.Conv_IntToDouble` _index) 10.0))
    (bind _outhit (`KismetSystemLibrary.SphereTraceSingle` :`Start` (`KismetMathLibrary.VLerp` (`SceneComponent.GetSocketLocation` _staticmesh "Trace_Start") (`SceneComponent.GetSocketLocation` _staticmesh "Trace_End") _returnvalue) :`End` (`KismetMathLibrary.VLerp` (`self.LastTraceStartLocation`) (`self.LastTraceEndLocation`) _returnvalue) :`Radius` (`self.TraceStep`) :`TraceChannel` "TraceTypeQuery1" :`DrawTime` 0.2))
    (`self.CacheTraceLoacations`)
    (bind (_bblockinghit _binitialoverlap _time _distance _location _impactpoint _normal _impactnormal _physmat _hitactor) (`GameplayStatics.BreakHitResult` _outhit))
    (`/Engine/EditorBlueprintResources/StandardMacros.IsValid` _hitactor
      (:`Is Valid`
        (`GameplayStatics.ApplyDamage` _hitactor 0.0 null self)))))

(event `CacheTraceLoacations`
  (bind _staticmesh (`self.StaticMesh`))
  (set `self.LastTraceStartLocation` (`SceneComponent.GetSocketLocation` _staticmesh "Trace_Start"))
  (set `self.LastTraceEndLocation` (`SceneComponent.GetSocketLocation` _staticmesh "Trace_End")))

(fn `UserConstructionScript`)