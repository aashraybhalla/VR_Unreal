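; Boat is a physics-driven rowboat that moves when paddled, registering itself as the VR pawn's Vehicle on BeginPlay.
; Each tick, while a valid Paddles reference reports being held, it reads the paddles' push velocity and origin.
; The inverted velocity drives two forces on the rowboat mesh, one at the push origin for turning and one central for propulsion, each with its own tuning multiplier.
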(event `self.ReceiveBeginPlay`
  (bind _returnvalue (`GameplayStatics.GetActorOfClass` "/Game/VRTemplate/Blueprints/VRPawn.VRPawn_C"))
  (set `/Game/VRTemplate/Blueprints/VRPawn.Vehicle` self _returnvalue))

(event `self.ReceiveTick`
  (params (DeltaSeconds :type "Float (single-precision)"))
  (bind _paddles (`self.Paddles`))
  (bind _sm_prop_rowboat (`self.SM_PROP_rowboat`))
  (bind (_velocity _origin) (`/Game/Fantastic_Village_Pack/blueprints/props/Paddles.GetPushVelocity` _paddles))
  (`/Engine/EditorBlueprintResources/StandardMacros.IsValid` _paddles
    (:`Is Valid`
      (if (`/Game/Fantastic_Village_Pack/blueprints/props/Paddles.IsHeld?` _paddles)
        (`PrimitiveComponent.AddForceAtLocation` _sm_prop_rowboat (* _velocity (`self.PaddlePushTorqueModifier`) -1.0) _origin "None")
        (`PrimitiveComponent.AddForce` _sm_prop_rowboat (* _velocity (`self.PaddlePushModifier`) -1.0) "None" false)))))

(fn `UserConstructionScript`)